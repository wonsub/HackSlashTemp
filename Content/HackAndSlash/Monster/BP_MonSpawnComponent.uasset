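; Spawner component that spawns a random monster around its owner every second, with no count limit.
; A looping timer calls DoSpawn, which picks a random DT_Monster row and spawns its class with the BT_Mon behavior tree.
; The row name then goes to SetMonStat on BP_MonseterBase.
; GetRandomCircleLocation rolls separate angles for X and Y, scaled by Radius times pi, so points scatter across a square rather than a circle.
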(event EventBeginPlay
  (Utilities|Time|SetTimerbyFunctionName 0 "DoSpawn" 1.0 true))

(event EventTick
  (params (DeltaSeconds :type Float%20%28single-precision%29)))

(fn DoSpawn
  (bind _outrownames (DataTable|GetDataTableRowNames "/Game/HackAndSlash/Monster/DT_Monster.DT_Monster"))
  (bind _output_get (LocalVariables|SetRowName (.OutItem (Utilities|Array|Random _outrownames))))
  (bind _returnvalue (Utilities|GetDataTableRow "/Game/HackAndSlash/Monster/DT_Monster.DT_Monster" _output_get)
    (:then
      (bind _returnvalue_2 (AI|SpawnAIFromClass (.MonsterClass (Utilities|Struct|BreakST_Monster _returnvalue)) "/Game/HackAndSlash/AI/BT_Mon.BT_Mon" (CallFunction|GetRandomCircleLocation) "0, 0, 0" false 0))
      (bind _asbp_monseter_base (Utilities|Casting|CastToBP_MonseterBase _returnvalue_2))
      (Default|SetMonStat _asbp_monseter_base (LocalVariables|GetRowName)))))

(fn GetRandomCircleLocation
  (bind _returnvalue (Math|Random|RandomFloatinRange 0.0 3.6e+02))
  (bind _radius (Variables|Default|GetRadius))
  (bind _returnvalue_2 (* _radius 3.141592))
  (LocalVariables|SetRand _returnvalue)
  (return (+ (Transformation|GetActorLocation (Components|GetOwner)) (Math|Vector|MakeVector (* (Math|Trig|Cos(Radians) _returnvalue) _returnvalue_2) (* (Math|Trig|Sin(Radians) _returnvalue) _returnvalue_2) 0.0))))