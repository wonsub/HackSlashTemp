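; BP_SKillMgr is a skill manager component that automatically casts its owner's skills whenever their cooldowns elapse.
; AddSkill looks up a DT_Skill row and stores it with its timer already at CoolTime, so it fires almost immediately.
; Tick advances each timer; once past CoolTime, it spawns the row's SkillClass at the owner's transform, passing the owning Character, and resets the timer.
; Adding and using skills print debug messages.
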(event EventBeginPlay)

(event EventTick
  (params (DeltaSeconds :type Float%20%28single-precision%29))
  (CallFunction|UpdateSkills DeltaSeconds))

(fn AddSkill
  (params (SkillRowName :type Name))
  (bind _returnvalue (Utilities|GetDataTableRow "/Game/HackAndSlash/Skills/DT_Skill.DT_Skill" SkillRowName)
    (:then
      (Utilities|Array|Add (Variables|Default|GetSkills) (Utilities|Struct|MakeST_CurSkill _returnvalue (.CoolTime (Utilities|Struct|BreakST_Skill _returnvalue))))
      (Development|PrintString (Utilities|String|Append "AddSkill - " (.Name (Utilities|Struct|BreakST_Skill _returnvalue))) true true "(R=0.000000,G=0.660000,B=1.000000,A=1.000000)" 2e+01))))

(fn UpdateSkills
  (params (DeltaSeconds :type Float%20%28double-precision%29))
  (for (_ _array_index) (Variables|Default|GetSkills)
    (CallFunction|UpdateSkillCoolTime (Utilities|Array|Get(acopy) (Variables|Default|GetSkills) _array_index) DeltaSeconds)))

(fn DoUseSkilll
  (params (CurSkill :type ST%20Cur%20Skill%20Structure))
  (bind _skilldata (Utilities|Struct|BreakST_CurSkill CurSkill))
  (bind _returnvalue (Components|GetOwner))
  ;[0.15 0.15 0.15 0.5] 로그
  (Development|PrintString (Utilities|String|Append "UseSkill - " (.name _skilldata)))
  (bind _ascharacter (Utilities|Casting|CastToCharacter _returnvalue))
  (Game|SpawnActorfromClass (.skillclass _skilldata) (Transformation|GetActorTransform _returnvalue) "Undefined" "MultiplyWithRoot" 0 _ascharacter 0))

(fn UpdateSkillCoolTime
  (params (CurSkill :type ST%20Cur%20Skill%20Structure%20%28by%20ref%29) (DeltaSeconds :type Float%20%28double-precision%29))
  (bind _structout (Utilities|Struct|SetmembersinST_CurSkill CurSkill (+ (.CurCoolTime (Utilities|Struct|BreakST_CurSkill CurSkill)) DeltaSeconds)))
  (if (> (.CurCoolTime (Utilities|Struct|BreakST_CurSkill _structout)) (.cooltime (.SkillData (Utilities|Struct|BreakST_CurSkill _structout))))
    (CallFunction|DoUseSkilll _structout)
    (Utilities|Struct|SetmembersinST_CurSkill _structout 0.0)))