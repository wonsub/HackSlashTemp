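; BP_ItemSpawnComponent is an actor component that keeps spawning random items around its owner.
; On BeginPlay it starts a looping one-second timer that calls DoSpanwnItem.
; Each call picks a random row from DT_Item and spawns that row's ItemClass at a random navigable point within a large radius of the owner, passing the row in as ItemData.
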(event EventBeginPlay
  (Utilities|Time|SetTimerbyFunctionName 0 "DoSpanwnItem" 1.0 true))

(fn DoSpanwnItem
  (bind _outrownames (DataTable|GetDataTableRowNames "/Game/HackAndSlash/Items/DT_Item.DT_Item"))
  (bind _output_get (LocalVariables|SetRandRowName (.OutItem (Utilities|Array|Random _outrownames))))
  (bind _returnvalue (Utilities|GetDataTableRow "/Game/HackAndSlash/Items/DT_Item.DT_Item" _output_get)
    (:then
      (bind _randomlocation (Class|NavigationSystemV1|GetRandomLocationinNavigableRadius (Transformation|GetActorLocation (Components|GetOwner)) 1e+04 0 0))
      (Game|SpawnActorfromClass (.ItemClass (Utilities|Struct|BreakST_ITem _returnvalue)) (Math|Transform|MakeTransform _randomlocation "0, 0, 0" "1.000000,1.000000,1.000000") "Undefined" "MultiplyWithRoot" 0 _returnvalue 0))))