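; Buff component for a hack-and-slash game that applies timed buffs and removes them when they expire.
; AddBuff looks up a DT_Buff row, stores it with an elapsed timer and applies its effect.
; Tick advances every timer, then removes expired entries one at a time, rescanning until none remain.
; Magnet is the only handled type, toggling a shared IsMagnet flag, so any Magnet expiry clears it.
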(event EventTick
  (params (DeltaSeconds :type Float%20%28single-precision%29))
  (CallFunction|UpdateBuff DeltaSeconds))

(fn AddBuff
  (params (RowName :type Name))
  (bind _returnvalue (Utilities|GetDataTableRow "/Game/HackAndSlash/Items/DT_Buff.DT_Buff" RowName)
    (:then
      (bind _returnvalue_2 (Utilities|Array|Add (Variables|Default|GetBuffs) (Utilities|Struct|MakeST_CurBuff _returnvalue 0.0)))
      (Development|PrintString (Utilities|String|Append "AddBuff - " (.Name (Utilities|Struct|BreakST_Buff _returnvalue))))
      (CallFunction|UseBuff (Utilities|Array|Get(acopy) (Variables|Default|GetBuffs) _returnvalue_2)))))

(fn UpdateBuff
  (params (DeltaSeconds :type Float%20%28double-precision%29))
  (for (_ _array_index) (Variables|Default|GetBuffs)
    (CallFunction|UpdateBuffCooltime (Utilities|Array|Get(acopy) (Variables|Default|GetBuffs) _array_index) DeltaSeconds))
  ;[0.15 0.15 0.15 0.5] 쿨타임 종료된 버프 정리
  (bind _removeindex (CallFunction|RemoveTimeOverBuffs :!label _label))
  (if (!= _removeindex -1)
    (goto _label)))

(fn RemoveTimeOverBuffs
  (for (_array_element _array_index) (Variables|Default|GetBuffs)
    (if (> (.CurCoolTime (Utilities|Struct|BreakST_CurBuff _array_element)) (.cooltime (.Buff (Utilities|Struct|BreakST_CurBuff _array_element))))
      (CallFunction|RemoveBuff _array_element)
      (Development|PrintString (Utilities|String|Append "Remove Buff - " (.name (.Buff (Utilities|Struct|BreakST_CurBuff _array_element)))) true true "(R=1.000000,G=0.016751,B=0.000000,A=1.000000)" 2e+01)
      (Utilities|Array|RemoveIndex (Variables|Default|GetBuffs) _array_index)
      (return _array_index)))
  (return -1))

(fn UpdateBuffCooltime
  (params (CurBuff :type ST%20Cur%20Buff%20Structure%20%28by%20ref%29) (DeltaSeconds :type Float%20%28double-precision%29%20%28by%20ref%29))
  (Utilities|FlowControl|Sequence
    (:then_0
      (Utilities|Struct|SetmembersinST_CurBuff CurBuff (+ (.CurCoolTime (Utilities|Struct|BreakST_CurBuff CurBuff)) DeltaSeconds)))))

(fn UseBuff
  (params (CurBuff :type ST%20Cur%20Buff%20Structure%20%28by%20ref%29))
  (Development|PrintString (Utilities|String|Append "Use Buff" (.name (.buff CurBuff))))
  (switch Utilities|FlowControl|Switch|SwitchonEN_BuffType (.bufftype (.buff CurBuff))
    (:NewEnumerator2
      (Variables|Default|SetIsMagnet true))))

(fn RemoveBuff
  (params (CurBuff :type ST%20Cur%20Buff%20Structure))
  (switch Utilities|FlowControl|Switch|SwitchonEN_BuffType (.bufftype (.buff CurBuff))
    (:NewEnumerator2
      (Variables|Default|SetIsMagnet false))))